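; Star actor that tints its Sphere component according to its size and a Temp value.
; On BeginPlay it sets the "Color" material parameter once, choosing between two palettes by a threshold on the actor's X scale.
; Smaller stars get a red-dominant color and larger ones a blue-dominant color, with channel values derived from Temp.
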(event `self.ReceiveBeginPlay`
  (bind _temp (`self.temp`))
  (bind _temp_2 (`self.temp`))
  (`MeshComponent.SetVectorParameterValueOnMaterials` (`self.Sphere`) "Color" (`KismetMathLibrary.SelectVector` (`KismetMathLibrary.MakeVector` (+ _temp_2 150.0) (- 20.0 (/ _temp_2 10.0))) (`KismetMathLibrary.MakeVector` 0.0 (/ _temp 5.0) (+ _temp 200.0)) (<= (* (.x (.scale (`self.GetTransform`))) 5.0) 200.0))))

(fn `UserConstructionScript`)