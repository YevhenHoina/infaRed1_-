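; Player-controlled space ship with twin-stick flight and aiming, plus unfinished procedural spawning of space scenery.
; BeginPlay disables capsule gravity, adds the Aiming input context and spawns one randomly placed, scaled Star.
; Left stick moves the ship in world XY and steps Core's yaw toward the stick angle; right stick steps both weapons likewise.
; Asteroid spawning on Tick is disconnected, and the construction script only randomizes the Star1 transform.
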(event `self.ReceiveBeginPlay`
  (`self.GigansGeneration`)
  (`PrimitiveComponent.SetEnableGravity` (`self.CapsuleComponent`) false)
  (set `self.FirstPos` (`self.GetTransform`))
  (bind _asplayer_controller (cast `PlayerController` (`self.GetController`)))
  (bind _returnvalue (pcsubsystem `EnhancedInputLocalPlayerSubsystem` _asplayer_controller))
  (`/Engine/EditorBlueprintResources/StandardMacros.IsValid` _returnvalue
    (:`Is Valid`
      (`EnhancedInputSubsystemInterface.AddMappingContext` _returnvalue "/Game/Blueprint/Aiming.Aiming" 0 (struct)))))

(event `self.ReceiveTick`
  (params (DeltaSeconds :type "Float (single-precision)")))

(event `EnhancedInput|/Game/Blueprint/LeftJoystick`
  (params (ActionValue :type "Vector2D Structure") (ElapsedSeconds :type "Float (double-precision)") (TriggeredSeconds :type "Float (double-precision)") (InputAction :type "InputAction Object Reference" :default "/Game/Blueprint/LeftJoystick.LeftJoystick"))
  (:`Triggered`
    (`self.SmoothRotation` ActionValue_Y ActionValue_X (`self.Core`))))

(event `EnhancedInput|/Game/Blueprint/RightJoystick`
  (params (ActionValue :type "Vector2D Structure") (ElapsedSeconds :type "Float (double-precision)") (TriggeredSeconds :type "Float (double-precision)") (InputAction :type "InputAction Object Reference" :default "/Game/Blueprint/RightJoystick.RightJoystick"))
  (:`Triggered`
    (`self.SmoothAim` ActionValue_Y ActionValue_X)))

(fn `CurrentCoordinates`
  (returns (ReturnValue :type "Vector Structure"))
  (return (`self.K2_GetActorLocation`)))

(fn `GameStarted`
  (params (DeltaTime :type "Float (double-precision)"))
  (locals (NewLocalVar :type Integer)))

(fn `Generation`)

(fn `GigansGeneration`
  (locals (CurrentLocation :type "Vector Structure" :default (0.0 0.0 0.0)))
  (bind _output_get (set `self.SecondPos` (`self.GetTransform`)))
  (bind _location (.location _output_get))
  (if (>= (`KismetMathLibrary.Vector_Distance` _location (.location (`self.FirstPos`))) (`self.GigantGenerationSpeed`))
    (set `self.FirstPos` (`self.GetTransform`)))
  (bind _output_get_2 (set `local.CurrentLocation` _location))
  (`|SpawnActorFromClass` "/Game/Blueprint/Star.Star_C" (`KismetMathLibrary.MakeTransform` (`KismetMathLibrary.MakeVector` (+ (.x _output_get_2) (* (`KismetMathLibrary.RandomFloatInRange` 15000.0 25000.0) (`KismetMathLibrary.SelectFloat` 1.0 -1.0 (`KismetMathLibrary.RandomBool`)))) (+ (.y _output_get_2) (`KismetMathLibrary.RandomFloatInRange` -25000.0 25000.0)) (+ (.z _output_get_2) (`KismetMathLibrary.SelectFloat` (`KismetMathLibrary.RandomFloatInRange` -1200.0 -800.0) (`KismetMathLibrary.RandomFloatInRange` 800.0 1200.0) (`KismetMathLibrary.RandomBool`)))) (struct) (* (`KismetMathLibrary.Vector_One`) (`KismetMathLibrary.RandomFloatInRange` 20.0 51.0))) "Undefined" "OverrideRootScale" null null))

(fn `SmoothAim`
  (params (X :type "Float (double-precision)") (Y :type "Float (double-precision)"))
  (bind _returnvalue (* Y -1.0))
  (bind _yaw (.yaw (`KismetMathLibrary.NormalizedDeltaRotator` (`KismetMathLibrary.MakeRotator` 0.0 0.0 (`KismetMathLibrary.DegAtan` (/ X _returnvalue))) (`SceneComponent.K2_GetComponentRotation` (`self.LeftWeapon`)))))
  (`KismetSystemLibrary.PrintString` (`KismetStringLibrary.Conv_DoubleToString` Y))
  (`SceneComponent.K2_AddWorldRotation` (`self.LeftWeapon`) (`KismetMathLibrary.SelectRotator` (struct :`Yaw` -1.0) (struct :`Yaw` 1.0) (select `bool` (< 0.0 _returnvalue) :`false` (< 0.0 _yaw) :`true` (> 0.0 _yaw))) false false)
  (`SceneComponent.K2_AddWorldRotation` (`self.RightWeapon`) (`KismetMathLibrary.SelectRotator` (struct :`Yaw` -1.0) (struct :`Yaw` 1.0) (select `bool` (< 0.0 _returnvalue) :`false` (< 0.0 _yaw) :`true` (> 0.0 _yaw))) false false))

(fn `SmoothRotation`
  (params (X :type "Float (double-precision)") (Y :type "Float (double-precision)") (Object1 :type "SceneComponent Object Reference"))
  (bind _enginespeed (`self.EngineSpeed`))
  (bind _yaw (.yaw (`KismetMathLibrary.NormalizedDeltaRotator` (`KismetMathLibrary.MakeRotator` 0.0 0.0 (`KismetMathLibrary.DegAtan` (/ X Y))) (`SceneComponent.K2_GetComponentRotation` (`local.Object1`)))))
  (`SceneComponent.K2_AddWorldRotation` (`local.Object1`) (select `bool` (< (`KismetMathLibrary.Abs` _yaw) 10.0) :`false` (`KismetMathLibrary.SelectRotator` (struct :`Yaw` -1.0) (struct :`Yaw` 1.0) (select `bool` (< (`local.Y`) 0.0) :`false` (< _yaw 0.0) :`true` (> _yaw 0.0)))) false false)
  (`self.K2_AddActorWorldTransform` (`KismetMathLibrary.MakeTransform` (`KismetMathLibrary.MakeVector` (* (`local.Y`) _enginespeed) (* (`local.X`) _enginespeed)))))

(fn `UserConstructionScript`
  (set `self.Star1` (`KismetMathLibrary.MakeTransform` (`KismetMathLibrary.MakeVector` (* (`KismetMathLibrary.RandomFloatInRange` 25600.0 64000.0) (`KismetMathLibrary.SelectFloat` 1.0 -1.0 (`KismetMathLibrary.RandomBool`))) (* (`KismetMathLibrary.RandomFloatInRange` 25600.0 64000.0) (`KismetMathLibrary.SelectFloat` 1.0 -1.0 (`KismetMathLibrary.RandomBool`))) (* (`KismetMathLibrary.RandomFloatInRange` 25600.0 64000.0) (`KismetMathLibrary.SelectFloat` 1.0 -1.0 (`KismetMathLibrary.RandomBool`)))) (struct) (* (`KismetMathLibrary.Vector_One`) (`KismetMathLibrary.RandomFloatInRange` 20.0 51.0)))))